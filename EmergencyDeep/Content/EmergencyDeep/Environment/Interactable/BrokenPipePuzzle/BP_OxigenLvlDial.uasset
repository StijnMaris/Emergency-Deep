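; Oxygen level dial in the broken pipe puzzle area that displays the game's current oxygen level.
; Every Tick it reads the oxygen level from BP_EDGameGameState, stores it in OxigenLvl and passes it to SetOxigen.
; SetOxigen treats the value as a percentage and slides the Pin component along its local Z axis within a clamped range.
; OxigenLvl has a RepNotify, but its handler is empty.
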(event `self.ReceiveBeginPlay`)

(event `self.ReceiveTick`
  (params (DeltaSeconds :type "Float (single-precision)"))
  (bind _asbp_edgame_game_state (cast `/Game/EmergencyDeep/Game/BP_EDGameGameState` (`GameplayStatics.GetGameState`)))
  ;[1 1 1] Comment
  (bind _output_get (set `self.OxigenLvl` (`EDGameGameState.GetOxygenLevel` _asbp_edgame_game_state)))
  (`self.SetOxigen` _output_get))

(event `SetOxigen`
  (params (Oxygen :type "Float (double-precision)"))
  (`SceneComponent.K2_SetRelativeLocation` (`self.Pin`) (`KismetMathLibrary.MakeVector` 0.0 4.0 (`KismetMathLibrary.FClamp` (* (/ Oxygen 100.0) 40.0) 4.0 40.0)) false false))

(fn `OnRep_OxigenLvl`)

(fn `UserConstructionScript`)