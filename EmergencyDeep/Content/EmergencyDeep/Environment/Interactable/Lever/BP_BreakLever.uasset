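; BP_BreakLever is an interactable lever that starts and stops movement through WorldControl.
; The top trigger starts movement only when the Engine's current failure is Idle, while the bottom trigger stops it, each playing its own click sound.
; Tick feeds the handle's pitch to LeverArrow and repeatedly stops movement while the engine failure is Shutdown.
; Handle move events start and stop a movement sound.
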(event `self.ReceiveTick`
  (params (DeltaSeconds :type "Float (single-precision)"))
  (`LeverArrowComponent.SetInputAngle` (`self.LeverArrow`) (.pitch (.rotation (`SceneComponent.GetRelativeTransform` (`self.HandleMesh`)))))
  (switch `EEngineFailureType` (`EngineControlPanel.CurrentFailure` (`self.Engine`))
    (:`EFT_Shutdown`
      (`WorldControlComponent.StopMove` (`self.WorldControl`)))))

(event `self.OnTopTriggerBegin_BP`
  (`AudioComponent.Play` (`self.SW_Click_02`) 0.0)
  (if (`|EnumEquality` (`EngineControlPanel.CurrentFailure` (`self.Engine`)) "EFT_Idle")
    (`WorldControlComponent.StartMove` (`self.WorldControl`))))

(event `self.OnBottomTriggerBegin_BP`
  (`AudioComponent.Play` (`self.SW_Click_01`) 0.0)
  (`WorldControlComponent.StopMove` (`self.WorldControl`)))

(event `self.OnHandleMoveBegin_BP`
  (`AudioComponent.Play` (`self.SW_Move`) 0.0))

(event `self.OnHandleMoveEnd_BP`
  (`AudioComponent.Stop` (`self.SW_Move`)))

(fn `UserConstructionScript`)