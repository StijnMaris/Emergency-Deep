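; Guide book page actor that shows the texture of the engine control panel's current puzzle template on its static mesh.
; On BeginPlay it caches the first BP_EngineControlPanel found in the level.
; Every Tick it fetches that panel's current template and, if valid, creates a dynamic material instance from the mesh's material, setting the ColorPallet parameter to the template's texture.
; The material is rebuilt each frame rather than on template change.
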(event `self.ReceiveBeginPlay`
  (bind _outactors (`GameplayStatics.GetAllActorsOfClass` "/Game/EmergencyDeep/Puzzles/BP_EngineControlPanel.BP_EngineControlPanel_C"))
  (if (> (`KismetArrayLibrary.Array_Length` _outactors) 0)
    (set `self.ControlPanel` (`|GetArrayItem` _outactors))))

(event `self.ReceiveTick`
  (params (DeltaSeconds :type "Float (single-precision)"))
  (bind _staticmesh (`self.StaticMesh`))
  (bind _returnvalue (`EngineControlPanel.GetCurrentTemplate` (`self.ControlPanel`)))
  (`/Engine/EditorBlueprintResources/StandardMacros.IsValid` _returnvalue
    (:`Is Valid`
      (bind _asbp_ecppuzzle_template_base (cast `/Game/EmergencyDeep/Puzzles/BP_ECPPuzzleTemplateBase` _returnvalue))
      (bind _returnvalue_2 (`PrimitiveComponent.CreateDynamicMaterialInstance` _staticmesh 0 (`PrimitiveComponent.GetMaterial` _staticmesh 0) "None"))
      (`MaterialInstanceDynamic.SetTextureParameterValue` _returnvalue_2 "ColorPallet" (`/Game/EmergencyDeep/Puzzles/BP_ECPPuzzleTemplateBase.TemplateTexture` _asbp_ecppuzzle_template_base))
      (`PrimitiveComponent.SetMaterial` _staticmesh 0 _returnvalue_2))))

(fn `UserConstructionScript`)