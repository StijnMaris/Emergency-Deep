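; Submarine steering wheel interactable that turns valve rotation into steering by rotating the world control.
; The valve-rotated event passes its delta angle to WorldControl only while the engine's current failure state is Idle.
; Each tick, it reads the total delta from the world generator and shows it on the S_Steering widget hosted in its widget component.
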(event `self.ReceiveTick`
  (params (DeltaSeconds :type "Float (single-precision)"))
  (bind _worldgenerator (`self.WorldGenerator`))
  (bind _ass_steering (cast `/Game/EmergencyDeep/Environment/Interactable/Steering_Wheel/S_Steering` (`WidgetComponent.GetUserWidgetObject` (`self.Widget`))))
  (`/Engine/EditorBlueprintResources/StandardMacros.IsValid` _worldgenerator
    (:`Is Valid`
      (bind _returnvalue (`WorldGenerator.GetTotalDelta` _worldgenerator))
      (`/Game/EmergencyDeep/Environment/Interactable/Steering_Wheel/S_Steering.SetSteering` _ass_steering _returnvalue))))

(event `self.OnValveRotated_BP`
  (params (deltaAngle :type "Float (single-precision)") (newAngle :type "Float (single-precision)"))
  (if (`|EnumEquality` (`EngineControlPanel.CurrentFailure` (`self.Engine`)) "EFT_Idle")
    (`WorldControlComponent.Rotate` (`self.WorldControl`) deltaAngle)))

(fn `UserConstructionScript`)