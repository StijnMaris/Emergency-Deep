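; Sonar table actor that displays detected sonar objects as colored widget dots.
; On each sonar refresh it rebuilds its widget components on BPSonar, placing each dot via CalculateDotPosition, rotated by the table's rotation plus a 90-degree yaw offset.
; Dot colors come from each detected actor's SonarDetectableObjectComponent.
; Tick copies BPSonar's PingAlpha into every dot's opacity, so the dots follow the ping.
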(event `self.ReceiveBeginPlay`)

(event `self.ReceiveTick`
  (params (DeltaSeconds :type "Float (single-precision)"))
  (for _array_element (`self.SonarWidgets`)
    (bind _returnvalue (`WidgetComponent.GetUserWidgetObject` _array_element))
    (bind (_r _g _b) (`KismetMathLibrary.BreakColor` (`UserWidget.ColorAndOpacity` _returnvalue)))
    (`UserWidget.SetColorAndOpacity` _returnvalue (`KismetMathLibrary.MakeColor` _r _g _b (`Sonar.PingAlpha` (`self.BP_Sonar`))))))

(fn `OnSonarRefresh`
  (params (SonarObjects :type "Array of SonarObject Structure"))
  (for _array_element (`self.SonarWidgets`)
    (`ActorComponent.K2_DestroyComponent` _array_element))
  (`KismetArrayLibrary.Array_Clear` (`self.SonarWidgets`))
  (for _array_element_2 SonarObjects
    (bind _returnvalue (`AddComponent|NODE_AddWidgetComponent-2` :`bManualAttachment` true))
    (`SceneComponent.K2_AttachToComponent` _returnvalue (`self.BP_Sonar`) "None" "SnapToTarget" "SnapToTarget" "SnapToTarget" true)
    (`KismetArrayLibrary.Array_Add` (`self.SonarWidgets`) _returnvalue)
    (bind _returnvalue_2 (`Sonar.CalculateDotPosition` (`self.BP_Sonar`) (`self.CircleRadius`) _array_element_2))
    (bind _returnvalue_3 (`WidgetComponent.GetUserWidgetObject` _returnvalue))
    (bind (_x _y) (`KismetMathLibrary.BreakVector2D` _returnvalue_2))
    (`Widget.SetRenderTranslation` _returnvalue_3 (`KismetMathLibrary.MakeVector2D` (.x (`KismetMathLibrary.GreaterGreater_VectorRotator` (`KismetMathLibrary.MakeVector` _x _y) (`KismetMathLibrary.MakeRotator` (.roll (`self.K2_GetActorRotation`)) (.pitch (`self.K2_GetActorRotation`)) (+ (.yaw (`self.K2_GetActorRotation`)) 90.0)))) (.y (`KismetMathLibrary.GreaterGreater_VectorRotator` (`KismetMathLibrary.MakeVector` _x _y) (`KismetMathLibrary.MakeRotator` (.roll (`self.K2_GetActorRotation`)) (.pitch (`self.K2_GetActorRotation`)) (+ (.yaw (`self.K2_GetActorRotation`)) 90.0))))))
    (`UserWidget.SetColorAndOpacity` _returnvalue_3 (`KismetMathLibrary.Conv_ColorToLinearColor` (`SonarDetectableObjectComponent.SonarPingColor` (`self.GetComponentByClass` (`.Actor` (break `SonarObject` _array_element_2)) "/Script/EmergencyDeep.SonarDetectableObjectComponent"))))))

(fn `UserConstructionScript`)