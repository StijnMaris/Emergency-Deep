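; Grabbable VR valve that the player handles with a motion controller.
; The construction script picks a random valve mesh and enables physics simulation on it.
; Grab and release events forward to the grippable mesh component through a physics handle, and Tick force-detaches it when the controller moves beyond ReleaseDistance.
; The actor's own attach, detach and gripped-query functions are stubs that return false.
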(event `self.ReceiveBeginPlay`)

(event `EDGrabInterface.OnGrab`
  (params (MotionController :type "SceneComponent Object Reference") (PhysicsHandle :type "PhysicsHandleComponent Object Reference") (GrabLocation :type "Vector Structure"))
  (bind _output_get (set `self.MotionController` MotionController))
  (bind _output_get_2 (set `self.PhysicsHandle` PhysicsHandle))
  (`GrippableStaticMeshComponent.AttachComponent` (`self.GrippableStaticMesh`) _output_get _output_get_2 GrabLocation))

(event `EDGrabInterface.OnGrabRelease`
  (params (PhysicsHandle :type "PhysicsHandleComponent Object Reference"))
  (`GrippableStaticMeshComponent.DettachComponent` (`self.GrippableStaticMesh`) PhysicsHandle)
  (set `self.MotionController` null)
  (set `self.PhysicsHandle` null))

(event `self.ReceiveTick`
  (params (DeltaSeconds :type "Float (single-precision)"))
  (`/Engine/EditorBlueprintResources/StandardMacros.IsValid` (`self.MotionController`)
    (:`Is Valid`
      (if (> (`KismetMathLibrary.VSize` (- (`SceneComponent.K2_GetComponentLocation` (`self.GrippableStaticMesh`)) (`SceneComponent.K2_GetComponentLocation` (`self.MotionController`)))) (`self.ReleaseDistance`))
        (set `self.MotionController` null)
        (`GrippableStaticMeshComponent.DettachComponent` (`self.GrippableStaticMesh`) (`self.PhysicsHandle`))
        (set `self.PhysicsHandle` null)))))

(fn `AttachActor`
  (params (MotionController :type "SceneComponent Object Reference") (ToAttachActor :type "SceneComponent Object Reference") (ToSimulateComponent :type "PrimitiveComponent Object Reference"))
  (returns (ReturnValue :type Boolean))
  (return false))

(fn `AttachComponent`
  (params (MotionController :type "SceneComponent Object Reference") (PhysicsHandle :type "PhysicsHandleComponent Object Reference") (GrabLocation :type "Vector Structure"))
  (returns (ReturnValue :type Boolean))
  (return false))

(fn `DettachActor`
  (params (ToDettachActor :type "SceneComponent Object Reference") (ToSimulateComponent :type "PrimitiveComponent Object Reference") (IsSimPhysics :type Boolean))
  (returns (ReturnValue :type Boolean))
  (return false))

(fn `DettachComponent`
  (params (PhysicsHandle :type "PhysicsHandleComponent Object Reference"))
  (returns (ReturnValue :type Boolean))
  (return false))

(fn `HasBeenGripped`
  (returns (ReturnValue :type Boolean))
  (return false))

(fn `UserConstructionScript`
  (bind _valvemeshes (`self.ValveMeshes`))
  (bind _grippablestaticmesh (`self.GrippableStaticMesh`))
  (`StaticMeshComponent.SetStaticMesh` _grippablestaticmesh (`|GetArrayItem` _valvemeshes (`KismetMathLibrary.RandomInteger` (`KismetArrayLibrary.Array_Length` _valvemeshes))))
  (`PrimitiveComponent.SetSimulatePhysics` _grippablestaticmesh true))