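; BP_ModuleBoxPin is an interior module box prop whose pin swings back and forth continuously.
; On BeginPlay it randomizes a time offset and a swing speed, so separate instances move out of sync.
; Each Tick advances the time by delta seconds and speed, then sets the Pin component's relative pitch to the sine of that time scaled by PinRange.
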(event `self.ReceiveBeginPlay`
  (set `self.TotalTime` (`KismetMathLibrary.RandomFloatInRange` 0.0 180.0))
  (set `self.PinSpeed` (`KismetMathLibrary.RandomFloatInRange` 0.1 5.0)))

(event `self.ReceiveTick`
  (params (DeltaSeconds :type "Float (single-precision)"))
  (bind _output_get (set `self.TotalTime` (+ (`self.TotalTime`) (* (`GameplayStatics.GetWorldDeltaSeconds`) (`self.PinSpeed`)))))
  (bind _output_get_2 (set `self.PinValue` (`KismetMathLibrary.Sin` _output_get)))
  (`SceneComponent.K2_SetRelativeRotation` (`self.Pin`) (`KismetMathLibrary.MakeRotator` 0.0 (+ (* _output_get_2 (`self.PinRange`)) 0.0)) false false))

(fn `UserConstructionScript`)