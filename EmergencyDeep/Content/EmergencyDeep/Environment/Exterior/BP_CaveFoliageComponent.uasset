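; BP_CaveFoliageComponent is a cave foliage component for the exterior environment that can be moved vertically and turned about the Z axis.
; Move adds a speed value to a stored height, while UpdateRotation replaces the stored yaw.
; Both events rebuild the world transform from those values, pinning X and Y to the world origin at unit scale, without sweep.
; It has no Tick logic, so movement depends on external calls.
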(event `self.Move`
  (params (Speed :type "Float (single-precision)"))
  (set `self.CurrentHeight` (+ (`self.CurrentHeight`) Speed))
  (`self.K2_SetWorldTransform` (`KismetMathLibrary.MakeTransform` (`KismetMathLibrary.MakeVector` 0.0 0.0 (`self.CurrentHeight`)) (`KismetMathLibrary.MakeRotator` 0.0 0.0 (`self.CurretRotation`))) :!label _label))

(event `self.UpdateRotation`
  (params (Rotation :type "Float (single-precision)"))
  (set `self.CurretRotation` Rotation)
  (goto _label))