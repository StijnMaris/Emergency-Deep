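; AI controller for the Kelp Dragon that runs its behavior tree on BeginPlay.
; Each tick it sets the CanSeeShip blackboard key when the pawn is within DistanceToSeeShip of the world origin, which stands in for the ship's position.
; While in that range, it also teleports the pawn down to Z zero whenever it is at or above that height.
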(event `self.ReceiveTick`
  (params (DeltaSeconds :type "Float (single-precision)"))
  (bind _returnvalue (`self.K2_GetPawn`))
  (bind _returnvalue_2 (>= (`self.DistanceToSeeShip`) (`KismetMathLibrary.VSize` (`self.K2_GetActorLocation` (`self.K2_GetPawn`)))))
  (`BlackboardComponent.SetValueAsBool` (`AIBlueprintHelperLibrary.GetBlackboard` null) "CanSeeShip" _returnvalue_2)
  (if (and _returnvalue_2 (>= (.z (.location (`self.GetTransform` _returnvalue))) 0.0))
    (`self.K2_SetActorLocation` _returnvalue (`KismetMathLibrary.MakeVector` (.x (.location (`self.GetTransform` _returnvalue))) (.y (.location (`self.GetTransform` _returnvalue)))) false true)))

(event `self.ReceiveBeginPlay`
  (`self.RunBehaviorTree` (`AIBlueprintHelperLibrary.GetAIController` self) "/Game/EmergencyDeep/AI/BehaviourTrees/BT_KelpDragon.BT_KelpDragon"))

(fn `UserConstructionScript`)