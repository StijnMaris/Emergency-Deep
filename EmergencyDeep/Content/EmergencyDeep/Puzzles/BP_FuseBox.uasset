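; BP_FuseBox is a puzzle fuse box that handles the audio for breaking and being kick-started.
; Breaking plays the Break sound, waits for its duration, stops the Loop sound, then calls the break event dispatcher.
; Kick-starting plays the Restart sound, waits for its duration, starts the Loop sound, then calls the kick-start event dispatcher.
; Both dispatcher calls are therefore timed to the length of their sound clips.
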(event `self.OnBreakFusebox_BP`
  (params (BrokenWires :type Boolean))
  (bind _break (`self.Break`))
  (`AudioComponent.Play` _break 0.0)
  (`KismetSystemLibrary.Delay` (`SoundBase.Duration` (`AudioComponent.Sound` _break)))
  (`AudioComponent.Stop` (`self.Loop`))
  (`self.OnBreakFuseBoxEventDispatcher`))

(event `self.OnKickStarted_BP`
  (bind _restart (`self.Restart`))
  (`AudioComponent.Play` _restart 0.0)
  (`KismetSystemLibrary.Delay` (`SoundBase.Duration` (`AudioComponent.Sound` _restart)))
  (`AudioComponent.Play` (`self.Loop`) 0.0)
  (`self.OnKickStartFuseBoxEventDispatcher`))

(fn `UserConstructionScript`)