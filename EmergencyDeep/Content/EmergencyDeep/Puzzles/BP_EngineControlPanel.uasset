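; Engine control panel puzzle actor that gives audio and screen feedback as the player restarts a failed engine.
; Parent-class events play sounds for engine failure, correct steps, mistakes, failed attempts and successful restart, with the running sound following the start sound after a delay.
; Failure and successful restart also call event dispatchers.
; Tick pushes the current screen number to a BP_NumberWidget on its widget component.
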(event `self.ReceiveTick`
  (params (DeltaSeconds :type "Float (single-precision)"))
  (`parent.ReceiveTick` DeltaSeconds)
  (bind _asbp_number_widget (cast `/Game/EmergencyDeep/Environment/Interactable/Engine_Control_Panel/BP_NumberWidget` (`WidgetComponent.GetUserWidgetObject` (`self.Widget`))))
  (`/Game/EmergencyDeep/Environment/Interactable/Engine_Control_Panel/BP_NumberWidget.SetNumber` _asbp_number_widget (`self.CurrentScreenNumber`)))

(event `self.OnNewEngineFailure_BP`
  (`AudioComponent.Stop` (`self.EngineRunning`))
  (`AudioComponent.Play` (`self.EngineStop`) 0.0)
  (`self.OnNewEngineFailureEventDispatcher`))

(event `self.OnCompleteFail_BP`
  (`AudioComponent.Play` (`self.RestartFailed`) 0.0))

(event `self.OnMadeMistake_BP`
  (`AudioComponent.Play` (`self.StepFailed`) 0.0))

(event `self.OnSequenceCorrect_BP`
  (`AudioComponent.Play` (`self.StepComplete`) 0.0))

(event `self.OnEngineRestartSuccesfull_BP`
  (bind _enginestart (`self.EngineStart`))
  (`AudioComponent.Play` (`self.SequenceComplete`) 0.0)
  (`AudioComponent.Play` _enginestart 0.0)
  (`KismetSystemLibrary.Delay` (`SoundBase.Duration` (`AudioComponent.Sound` _enginestart)))
  (`AudioComponent.Play` (`self.EngineRunning`) 0.0)
  (`self.OnEngineRestartSucceFullEventDispatcher`))

(fn `UserConstructionScript`)