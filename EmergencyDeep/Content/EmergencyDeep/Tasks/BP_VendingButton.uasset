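; BP_VendingButton is a toggleable button, named for a vending machine, with an LED and point light showing its state.
; Every tick, ToggleLight sets the LED material color and light color to green when toggled, red otherwise.
; After a short delay on BeginPlay, it forces the toggle off as a collision workaround and sets LED intensity.
; The pull and release events are empty.
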(event `self.ReceiveTick`
  (params (DeltaSeconds :type "Float (single-precision)"))
  (`self.Toggle Light`))

(event `self.OnPullButtonPulled_BP`)

(event `self.OnPullButtonReleased_BP`)

(event `Toggle Light`
  (bind _led (`self.Led`))
  (bind _pointlight (`self.PointLight`))
  ;[1 1 1] LightControl
  (if (`self.Toggled`)
    (`MeshComponent.SetVectorParameterValueOnMaterials` _led "Color" (0.0 1.0 0.0))
    (`LightComponent.SetLightColor` _pointlight (struct :`G` 1.0 :`B` 0.006993 :`A` 1.0) true)
    (else
      (`MeshComponent.SetVectorParameterValueOnMaterials` _led "Color" (1.0 0.0 0.0))
      (`LightComponent.SetLightColor` _pointlight (struct :`R` 1.0 :`A` 1.0) true))))

(event `self.ReceiveBeginPlay`
  ;[1 1 1] toggle vs collision fix
  (`KismetSystemLibrary.Delay` 0.2)
  (`self.SetToggle` false)
  (`self.Toggle Light`)
  (`MeshComponent.SetScalarParameterValueOnMaterials` (`self.Led`) "Intensity" 4.0))

(fn `UserConstructionScript`)