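; BP_WhaleSpline is a creature actor that moves a configurable fish or whale mesh along a spline.
; On BeginPlay a timeline, with play rate set by FishSpeed, drives the mesh's position and yaw-corrected rotation along the path at FishSize scale.
; Each update also copies that position to SonarDetectableObject's override location.
; The construction script assigns the mesh and creates a dynamic material whose FishSpeed parameter gets random variation.
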(event `self.ReceiveBeginPlay`
  (bind _spline (`self.Spline`))
  (`TimelineComponent.SetPlayRate` (`self.Timeline_0`) (`self.FishSpeed`))
  (bind (_direction _animalpha) (`Timeline|Timeline_0`)
    (:`Update`
      (bind _returnvalue (* (`SplineComponent.GetSplineLength` _spline) _animalpha))
      (bind _returnvalue_2 (`SplineComponent.GetLocationAtDistanceAlongSpline` _spline _returnvalue "World"))
      (`SceneComponent.K2_SetWorldTransform` (`self.StaticMesh`) (`KismetMathLibrary.MakeTransform` _returnvalue_2 (`KismetMathLibrary.MakeRotator` (.roll (`SplineComponent.GetRotationAtDistanceAlongSpline` _spline _returnvalue "World")) (.pitch (`SplineComponent.GetRotationAtDistanceAlongSpline` _spline _returnvalue "World")) (+ (.yaw (`SplineComponent.GetRotationAtDistanceAlongSpline` _spline _returnvalue "World")) -90.0)) (`KismetMathLibrary.Conv_DoubleToVector` (`self.FishSize`))) false false)
      (set `SonarDetectableObjectComponent.OverrideLocation` _returnvalue_2 (`self.SonarDetectableObject`)))))

(fn `UserConstructionScript`
  (bind _speedrandomvar (`self.SpeedRandomVar`))
  (bind _fishmesh (`self.Fishmesh`))
  (bind _staticmesh (`self.StaticMesh`))
  (`StaticMeshComponent.SetStaticMesh` _staticmesh _fishmesh)
  (bind _returnvalue (`PrimitiveComponent.CreateDynamicMaterialInstance` _staticmesh 0 (`StaticMesh.GetMaterial` _fishmesh 0) "None"))
  (`MaterialInstanceDynamic.SetScalarParameterValue` _returnvalue "FishSpeed" (+ (`self.FishSpeed`) (`KismetMathLibrary.RandomFloatInRange` (* _speedrandomvar -1.0) _speedrandomvar))))