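; Fish school actor that moves a group of fish meshes along a spline, each trailing a bubble emitter.
; The construction script adds separate static mesh components with random position offsets and speeds, feeding speed into dynamic materials for animation.
; One timeline places every fish at the same spline distance plus its offset, yawed -90 degrees.
; Its play rate is overwritten per fish each update, so individual speeds don't separate their movement.
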(event `self.ReceiveBeginPlay`
  (bind _spline (`self.Spline`))
  (`|ExecutionSequence`
    (:`then_0`
      (for _array_element (`self.FishArray`)
        (`GameplayStatics.SpawnEmitterAttached` "/Game/EmergencyDeep/FX/Bubbles/P_FishBubbles.P_FishBubbles" _array_element)))
    (:`then_1`
      (bind (_direction _animalpha) (`Timeline|Timeline_0`)
        (:`Update`
          (for (_array_element_2 _array_index) (`self.FishArray`)
            (`TimelineComponent.SetPlayRate` (`self.Timeline_0`) (`|GetArrayItem` (`self.Fish Speed Random`) _array_index))
            (bind _returnvalue (* (`SplineComponent.GetSplineLength` _spline) _animalpha))
            (`SceneComponent.K2_SetWorldTransform` _array_element_2 (`KismetMathLibrary.MakeTransform` (+ (.location (`|GetArrayItem` (`self.fishTranform`) _array_index)) (`SplineComponent.GetLocationAtDistanceAlongSpline` _spline _returnvalue "World")) (`KismetMathLibrary.MakeRotator` (.roll (`SplineComponent.GetRotationAtDistanceAlongSpline` _spline _returnvalue "World")) (.pitch (`SplineComponent.GetRotationAtDistanceAlongSpline` _spline _returnvalue "World")) (+ (.yaw (`SplineComponent.GetRotationAtDistanceAlongSpline` _spline _returnvalue "World")) -90.0)) (`KismetMathLibrary.Conv_DoubleToVector` (`self.FishSize`))) false false)))))))

(fn `UserConstructionScript`
  (bind _speed_random_var (`self.Speed random var`))
  (bind _spawnrange (`self.SpawnRange`))
  (bind _returnvalue (* _spawnrange -1.0))
  (for _ (range (`self.FishAmount`))
    (bind _returnvalue_2 (`AddComponent|NODE_AddStaticMeshComponent-1`))
    (`KismetArrayLibrary.Array_Add` (`self.FishArray`) _returnvalue_2)
    (`StaticMeshComponent.SetStaticMesh` _returnvalue_2 (`self.Fish mesh`)))
  (for (_array_element _array_index) (`self.FishArray`)
    (bind _returnvalue_3 (`PrimitiveComponent.CreateDynamicMaterialInstance` _array_element 0 (`PrimitiveComponent.GetMaterial` _array_element 0) "None"))
    (`KismetArrayLibrary.Array_Add` (`self.Fish Speed Random`) (+ (`self.FishSpeed`) (`KismetMathLibrary.RandomFloatInRange` (* _speed_random_var -1.0) _speed_random_var)))
    (`MaterialInstanceDynamic.SetScalarParameterValue` _returnvalue_3 "FishSpeed" (* (`|GetArrayItem` (`self.Fish Speed Random`) _array_index) (`self.Fish anim speed`)))
    (`KismetArrayLibrary.Array_Add` (`self.fishTranform`) (`KismetMathLibrary.MakeTransform` (`KismetMathLibrary.MakeVector` (`KismetMathLibrary.RandomFloatInRange` _returnvalue _spawnrange) (`KismetMathLibrary.RandomFloatInRange` _returnvalue _spawnrange) (`KismetMathLibrary.RandomFloatInRange` _returnvalue _spawnrange))))))