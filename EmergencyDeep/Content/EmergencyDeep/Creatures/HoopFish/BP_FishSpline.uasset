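; BP_FishSpline is a creature actor that moves a fish particle system along a spline, filed under HoopFish.
; On BeginPlay it starts a timeline with play rate set by FishSpeed.
; Each update maps the timeline alpha to a distance along the spline and sets the particle system's world transform there.
; Rotation follows the spline with a -90 degree yaw offset, and scale stays at one.
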(event `self.ReceiveBeginPlay`
  (bind _spline (`self.Spline`))
  (`TimelineComponent.SetPlayRate` (`self.Timeline_0`) (`self.FishSpeed`))
  (bind (_direction _animalpha) (`Timeline|Timeline_0`)
    (:`Update`
      (bind _returnvalue (* (`SplineComponent.GetSplineLength` _spline) _animalpha))
      (`SceneComponent.K2_SetWorldTransform` (`self.ParticleSystem`) (`KismetMathLibrary.MakeTransform` (`SplineComponent.GetLocationAtDistanceAlongSpline` _spline _returnvalue "World") (`KismetMathLibrary.MakeRotator` (.roll (`SplineComponent.GetRotationAtDistanceAlongSpline` _spline _returnvalue "World")) (.pitch (`SplineComponent.GetRotationAtDistanceAlongSpline` _spline _returnvalue "World")) (+ (.yaw (`SplineComponent.GetRotationAtDistanceAlongSpline` _spline _returnvalue "World")) -90.0))) false false))))

(fn `UserConstructionScript`)