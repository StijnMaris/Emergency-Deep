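; BP_EDGameGameState is the game state Blueprint for EmergencyDeep, handling what happens when the game ends.
; OnGameOverBP prints a debug "GAME OVER", appends the score to the player character's GameOverText and makes it visible.
; After a delay it opens L_MainMenu; an unconnected debug branch that would clear the game-over flag never runs.
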(event `self.ReceiveBeginPlay`)

(event `self.OnGameOver_BP`
  (`KismetSystemLibrary.PrintString` "GAME OVER" true true (struct :`R` 1.0 :`A` 1.0) 20000.0)
  (bind _asbp_edplayer_character (cast `/Game/EmergencyDeep/Characters/BP_EDPlayerCharacter` (`GameplayStatics.GetPlayerPawn` 0)))
  (bind _gameovertext (`/Game/EmergencyDeep/Characters/BP_EDPlayerCharacter.GameOverText` _asbp_edplayer_character))
  (`TextRenderComponent.K2_SetText` _gameovertext (`KismetTextLibrary.Conv_StringToText` (`KismetStringLibrary.Concat_StrStr` (`KismetTextLibrary.Conv_TextToString` (`TextRenderComponent.Text` _gameovertext)) (`KismetTextLibrary.Conv_TextToString` (`KismetTextLibrary.Conv_IntToText` (`self.GetScore`))))))
  (`SceneComponent.SetVisibility` _gameovertext true false)
  (`KismetSystemLibrary.Delay` 30.0)
  (`GameplayStatics.OpenLevel` "L_MainMenu"))

(fn `UserConstructionScript`)