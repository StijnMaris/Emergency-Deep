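; Test VR pickup actor that toggles between held and released when a motion controller's side grip fires.
; OnSideGrip asks its GrippableStaticMesh whether it is gripped, then either attaches the actor's root to the controller or detaches it with physics simulation on.
; The grip logic lives on the mesh component; the actor's own attach, detach and HasBeenGripped functions are stubs returning false.
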(event `EDGrabInterface.OnSideGrip`
  (params (MotionController :type "SceneComponent Object Reference") (PhysicsHandle :type "PhysicsHandleComponent Object Reference") (GrabLocation :type "Vector Structure"))
  (bind _returnvalue (`self.K2_GetRootComponent`))
  (bind _grippablestaticmesh (`self.GrippableStaticMesh`))
  (bind _grippablestaticmesh_2 (`self.GrippableStaticMesh`))
  (if (`GrippableStaticMeshComponent.HasBeenGripped` _grippablestaticmesh)
    (`GrippableStaticMeshComponent.DettachActor` _grippablestaticmesh_2 _returnvalue _grippablestaticmesh_2 true)
    (else
      (`GrippableStaticMeshComponent.AttachActor` _grippablestaticmesh MotionController _returnvalue _grippablestaticmesh))))

(fn `AttachActor`
  (params (MotionController :type "SceneComponent Object Reference") (ToAttachActor :type "SceneComponent Object Reference") (ToSimulateComponent :type "PrimitiveComponent Object Reference"))
  (returns (ReturnValue :type Boolean))
  (return false))

(fn `AttachComponent`
  (params (MotionController :type "SceneComponent Object Reference") (PhysicsHandle :type "PhysicsHandleComponent Object Reference") (GrabLocation :type "Vector Structure"))
  (returns (ReturnValue :type Boolean))
  (return false))

(fn `DettachActor`
  (params (ToDettachActor :type "SceneComponent Object Reference") (ToSimulateComponent :type "PrimitiveComponent Object Reference") (IsSimPhysics :type Boolean))
  (returns (ReturnValue :type Boolean))
  (return false))

(fn `DettachComponent`
  (params (PhysicsHandle :type "PhysicsHandleComponent Object Reference"))
  (returns (ReturnValue :type Boolean))
  (return false))

(fn `HasBeenGripped`
  (returns (ReturnValue :type Boolean))
  (return false))

(fn `UserConstructionScript`)